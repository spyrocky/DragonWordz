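; BP_HealthPickUp is a one-use health pickup for the wizard player.
; When a Player-tagged actor overlaps its Box, it casts to BP_WizardPlayer and calls IncreateHealth on the BPPlayerStat component with 25.
; It spawns a heal particle, plays a pop sound, shows a popup and destroys itself.
; The popup text claims +20, unlike the amount applied, and an unconnected delayed-destroy branch never runs.
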(event OnComponentBeginOverlap(Box)
  (params (OverlappedComponent :type Primitive%20Component%20Object%20Reference) (OtherActor :type Actor%20Object%20Reference) (OtherComp :type Primitive%20Component%20Object%20Reference) (OtherBodyIndex :type Integer) (bFromSweep :type Boolean) (SweepResult :type Hit%20Result%20Structure%20%28by%20ref%29))
  (if (Actor|ActorHasTag OtherActor "Player")
    (bind _asbp_wizard_player (Utilities|Casting|CastToBP_WizardPlayer OtherActor))
    (Default|IncreateHealth (Variables|/Game/DragonWord/Player/BP_WizardPlayer.BP_WizardPlayer_C|GetBP_PlayerStat _asbp_wizard_player) 25.0)
    (Effects|SpawnEmitteratLocation "/Game/InfinityBladeEffects/Effects/FX_Monsters/FX_Monster_Ausar/P_AU_Heal_01.P_AU_Heal_01" (Transformation|GetActorLocation) "0, 0, 0" "2.000000,2.000000,2.000000")
    (Utilities|IsValid self
      (:Is%20Valid
        (Audio|PlaySound2D "/Game/Interface_And_Item_Sounds/Cues/Abstract_Pop_05_Cue.Abstract_Pop_05_Cue" 1.0 1.0 0.0 0 0)
        (Default|AddShowNotiPopUp _asbp_wizard_player "Wow! Health point + 20 ")
        (Actor|DestroyActor)))))

(event EventBeginPlay)

(event Collision|EventActorBeginOverlap
  (params (OtherActor :type Actor%20Object%20Reference)))

(event EventTick
  (params (DeltaSeconds :type Float%20%28single-precision%29)))

(fn ConstructionScript)