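; Cute Creature variant of the melee enemy base, supplying its attacks, movement speeds, bandage mesh and death animation.
; The bandage mesh follows the main mesh's pose via leader pose.
; INTAttacking randomly picks a normal or jump attack for Attacks, and speed events switch between idle and run walk speeds.
; The health component's HitAnim event plays the Attack1 montage, then restores walking mode on completion.
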(event HitAnim(BPC_Enemy_Health)
  ;[1 1 1] Damage
  (Animation|Montage|PlayMontage (Variables|Character|GetMesh) "/Game/DragonWord/Enemies/Enemy_Blueprint/CuteCreature/AM_Cute_Attack1.AM_Cute_Attack1"
    (:OnCompleted
      (Pawn|Components|CharacterMovement|SetMovementMode (Variables|Character|GetCharacterMovement) "MOVE_Walking" 0))))

(event EventBeginPlay
  (|CallParentFunction)
  ;[1 1 1] Make the optional meshes to use the same skeleton as Main Mesh
  (Components|SkinnedMesh|SetLeaderPoseComponent (Variables|Default|GetSK_Bandage) (Variables|Character|GetMesh) false false))

(event Collision|EventActorBeginOverlap
  (params (OtherActor :type Actor%20Object%20Reference))
  (|CallParentFunction OtherActor) ; This node is disabled and will not be called.\nDrag off pins to build functionality.
)

(event EventTick
  (params (DeltaSeconds :type Float%20%28single-precision%29))
  (|CallParentFunction DeltaSeconds) ; This node is disabled and will not be called.\nDrag off pins to build functionality.
)

(event EventINTAttacking
  (CallFunction|Attacks (Utilities|Select :Index (Math|Random|RandomIntegerinRange 0 1) :Option%200 (Variables|Default|GetAttack%20Anim) :Option%201 (Variables|Default|GetJump%20Attack%20Anim))))

(event EventChangeSpeedIdle
  (Variables|/Script/Engine.CharacterMovementComponent|SetMaxWalkSpeed (Variables|Character|GetCharacterMovement) 5e+02))

(event EventChangeSpeedRun
  (Variables|/Script/Engine.CharacterMovementComponent|SetMaxWalkSpeed (Variables|Character|GetCharacterMovement) 1.1e+03))

(fn ConstructionScript
  (|CallParentFunction)
  (Variables|Default|SetDeathAnimation "/Game/DragonWord/Enemies/Enemy_Blueprint/CuteCreature/AM_Cute_Die.AM_Cute_Die"))