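; Enemy spawner point that places BP_EnemyBase actors at random navigable locations and sets itself as their origin.
; FirstSpawn and RespawnEnemies share a recursive loop that fills up to a maximum count, and each melee spawn adds two nearby minions outside that count.
; Leaving the cull sphere starts a delayed respawn timer, while entry by a specific actor class cancels it.
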(event OnComponentEndOverlap(CullRespawnRadius)
  (params (OverlappedComponent :type Primitive%20Component%20Object%20Reference) (OtherActor :type Actor%20Object%20Reference) (OtherComp :type Primitive%20Component%20Object%20Reference) (OtherBodyIndex :type Integer))
  (Variables|Components|SetCanRespawn? true)
  (bind _returnvalue (Utilities|Time|SetTimerbyFunctionName 0 "RespawnEnemies" 9e+01))
  (Variables|Components|SetTimer _returnvalue))

(event OnComponentBeginOverlap(CullRespawnRadius)
  (params (OverlappedComponent :type Primitive%20Component%20Object%20Reference) (OtherActor :type Actor%20Object%20Reference) (OtherComp :type Primitive%20Component%20Object%20Reference) (OtherBodyIndex :type Integer) (bFromSweep :type Boolean) (SweepResult :type Hit%20Result%20Structure%20%28by%20ref%29))
  (if (== (Utilities|GetClass OtherActor) 0)
    (Variables|Components|SetCanRespawn? false)
    (Utilities|Time|ClearTimerbyFunctionName 0 "RespawnEnemies")))

(event Custom|FirstSpawn
  (if (< (Variables|Components|GetCurrentSpawnCount) (Variables|Components|GetMaxSpawnCount))
    (bind _randomlocation (Class|NavigationSystemV1|GetRandomLocationinNavigableRadius (Transformation|GetActorLocation) (Variables|Components|GetRespawnRadius) 0 0))
    (bind _returnvalue (Game|SpawnActorfromClass (Variables|Components|GetSpawnerActorType) (Math|Transform|MakeTransform _randomlocation "0, 0, 0" "1.000000,1.000000,1.000000") "AdjustIfPossibleButAlwaysSpawn" 0 0))
    (bind _asbp_enemy_base (Utilities|Casting|CastToBP_EnemyBase _returnvalue))
    (Utilities|IsValid _asbp_enemy_base
      (:Is%20Valid
        (Variables|/Game/DragonWord/Enemies/BP_EnemyBase.BP_EnemyBase_C|SetOrigin _asbp_enemy_base self)
        (Math|Integer|IncrementInt (Variables|Components|GetCurrentSpawnCount)
          (:%20%20
            (if (== (Variables|Components|GetSpawnerActorType) "/Game/DragonWord/Enemies/BP_EnemyBase_Malee.BP_EnemyBase_Malee_C")
              (Variables|/Game/DragonWord/Enemies/BP_EnemyBase.BP_EnemyBase_C|SetOriginDistance _asbp_enemy_base 0.0)
              (CallFunction|SpawnMinions (Transformation|GetActorLocation _returnvalue))
              (CallFunction|SpawnMinions (Transformation|GetActorLocation _returnvalue)))
            (if (Variables|Components|GetFirstSpawn?)
              ;[1 1 1] Continue to spawn the first wave (On begin play)
              (CallFunction|FirstSpawn)
              (else
                ;[1 1 1] Respawn Enemies as Normal
                (CallFunction|RespawnEnemies))))))
      (:Is%20Not%20Valid
        (Actor|DestroyActor _returnvalue)))
    (else
      (Variables|Components|SetCanRespawn? false)
      (Variables|Components|SetFirstSpawn? false))))

(event Custom|RespawnEnemies
  (if (Variables|Components|GetCanRespawn?)
    (if (< (Variables|Components|GetCurrentSpawnCount) (Variables|Components|GetMaxSpawnCount))
      (bind _randomlocation (Class|NavigationSystemV1|GetRandomLocationinNavigableRadius (Transformation|GetActorLocation) (Variables|Components|GetRespawnRadius) 0 0))
      (bind _returnvalue (Game|SpawnActorfromClass (Variables|Components|GetSpawnerActorType) (Math|Transform|MakeTransform _randomlocation "0, 0, 0" "1.000000,1.000000,1.000000") "AdjustIfPossibleButAlwaysSpawn" 0 0))
      (bind _asbp_enemy_base (Utilities|Casting|CastToBP_EnemyBase _returnvalue))
      (Utilities|IsValid _asbp_enemy_base
        (:Is%20Valid
          (Variables|/Game/DragonWord/Enemies/BP_EnemyBase.BP_EnemyBase_C|SetOrigin _asbp_enemy_base self)
          (Math|Integer|IncrementInt (Variables|Components|GetCurrentSpawnCount)
            (:%20%20
              (if (== (Variables|Components|GetSpawnerActorType) "/Game/DragonWord/Enemies/BP_EnemyBase_Malee.BP_EnemyBase_Malee_C")
                (Variables|/Game/DragonWord/Enemies/BP_EnemyBase.BP_EnemyBase_C|SetOriginDistance _asbp_enemy_base 0.0)
                (CallFunction|SpawnMinions (Transformation|GetActorLocation _returnvalue))
                (CallFunction|SpawnMinions (Transformation|GetActorLocation _returnvalue)))
              (if (Variables|Components|GetFirstSpawn?)
                ;[1 1 1] Continue to spawn the first wave (On begin play)
                (CallFunction|FirstSpawn)
                (else
                  ;[1 1 1] Respawn Enemies as Normal
                  (CallFunction|RespawnEnemies))))))
        (:Is%20Not%20Valid
          (Actor|DestroyActor _returnvalue)))
      (else
        (Variables|Components|SetCanRespawn? false)
        (Variables|Components|SetFirstSpawn? false)))))

(event Custom|SpawnMinions
  (params (ParentLocation :type Vector))
  (bind _randomlocation (Class|NavigationSystemV1|GetRandomLocationinNavigableRadius ParentLocation 3.5e+02 0 0))
  (bind _returnvalue (Game|SpawnActorfromClass (Variables|Components|GetSpawnerActorType) (Math|Transform|MakeTransform _randomlocation "0, 0, 0" "1.000000,1.000000,1.000000") "AdjustIfPossibleButAlwaysSpawn" 0 0))
  (bind _asbp_enemy_base (Utilities|Casting|CastToBP_EnemyBase _returnvalue))
  (Utilities|IsValid _asbp_enemy_base
    (:Is%20Valid
      (Variables|/Game/DragonWord/Enemies/BP_EnemyBase.BP_EnemyBase_C|SetOrigin _asbp_enemy_base self)
      (Variables|/Game/DragonWord/Enemies/BP_EnemyBase.BP_EnemyBase_C|SetOriginDistance _asbp_enemy_base 5e+03))
    (:Is%20Not%20Valid
      (Actor|DestroyActor _returnvalue))))

(event EventBeginPlay)

(event Collision|EventActorBeginOverlap
  (params (OtherActor :type Actor%20Object%20Reference)))

(event EventTick
  (params (DeltaSeconds :type Float%20%28single-precision%29)))

(fn ConstructionScript
  (if (Variables|Components|GetShortenRadius?)
    (Components|Sphere|SetSphereRadius (Variables|Default|GetCullRespawnRadius) 6.5e+03 true)))

(fn ShortenRadius)