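; BPC_Enemy_Health is a component that tracks an enemy's health and death state.
; Tick, rather than the empty BeginPlay, sets Health to MaxHealth and binds the owner's OnTakeAnyDamage, so both repeat every frame.
; Damage lowers Health until IsDead is set, calling ReceivingDamage and HitAnim while health remains, or DeathAnim and Death at zero or below.
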(event Custom|OnTakeAnyDamage_Event
  (params (DamagedActor :type Actor%20Object%20Reference) (Damage :type Float%20%28single-precision%29) (DamageType :type Damage%20Type%20Object%20Reference) (InstigatedBy :type Controller%20Object%20Reference) (DamageCauser :type Actor%20Object%20Reference))
  (Variables|Default|SetDamage Damage)
  (if (not (Variables|Default|GetisDead?))
    (bind _output_get (Variables|Default|SetHealth (- (Variables|Default|GetHealth) Damage)))
    (if (<= _output_get 0.0)
      (Variables|Default|SetisDead? true)
      (Utilities|FlowControl|Sequence
        (:then_0
          (Default|CallDeathAnim))
        (:then_1
          (Default|CallDeath)))
      (else
        (Utilities|FlowControl|Sequence
          (:then_0
            (Default|CallReceivingDamage))
          (:then_1
            (Default|CallHitAnim)))))))

(event EventTick
  (params (DeltaSeconds :type Float%20%28single-precision%29))
  (Variables|Default|SetHealth (Variables|Default|GetMax%20Health))
  (EventDispatchers|AssignOnTakeAnyDamage (Components|GetOwner) (delegate Custom|OnTakeAnyDamage_Event)))

(event EventBeginPlay)