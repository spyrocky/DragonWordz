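; BP_EnemyBase is the base enemy Blueprint, with a health component and a health widget.
; On BeginPlay it casts its widget to HUD_EnemiesHealth, caches it, and sets it from the BPCEnemyHealth component's current and max health.
; It then caches the player pawn as BP_WizardPlayer.
; Tick, overlap and construction script are empty, and the graph shows no health updates after spawn.
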(event Collision|EventActorBeginOverlap
  (params (OtherActor :type Actor%20Object%20Reference)))

(event EventTick
  (params (DeltaSeconds :type Float%20%28single-precision%29)))

(event EventBeginPlay
  (bind _bpc_enemy_health (Variables|Default|GetBPC_Enemy_Health))
  ;[0.6079 1 0.7411] Event Begin
  (Utilities|FlowControl|Sequence
    (:then_0
      (bind _ashud_enemies_health (Utilities|Casting|CastToHUD_EnemiesHealth (UserInterface|GetWidget (Variables|Default|GetWidget))))
      (bind _output_get (Variables|Default|SetAs%20WB%20Health _ashud_enemies_health))
      (Default|SetHealth _output_get (Variables|/Game/DragonWord/Enemies/Component/BPC_Enemy_Health.BPC_Enemy_Health_C|GetMax%20Health _bpc_enemy_health) (Variables|/Game/DragonWord/Enemies/Component/BPC_Enemy_Health.BPC_Enemy_Health_C|GetHealth _bpc_enemy_health)))
    (:then_1
      (bind _asbp_wizard_player (Utilities|Casting|CastToBP_WizardPlayer (Game|Player|GetPlayerPawn 0)))
      (Variables|Default|SetAs%20BP%20Wizard%20Player _asbp_wizard_player))))

(fn ConstructionScript)