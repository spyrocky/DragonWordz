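; Melee enemy Blueprint that sets its enemy type on BeginPlay and deals contact damage through an attack hitbox.
; MeleeHitBoxOn and MeleeHitBoxOff events toggle MeleeAttackBox between query-only and no collision, opening and closing the attack window.
; Any actor that begins overlapping the box takes damage equal to the Damage value from BPCEnemyHealth, with no target filtering.
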(event OnComponentBeginOverlap(MeleeAttackBox)
  (params (OverlappedComponent :type Primitive%20Component%20Object%20Reference) (OtherActor :type Actor%20Object%20Reference) (OtherComp :type Primitive%20Component%20Object%20Reference) (OtherBodyIndex :type Integer) (bFromSweep :type Boolean) (SweepResult :type Hit%20Result%20Structure%20%28by%20ref%29))
  (Game|Damage|ApplyDamage OtherActor (Variables|/Game/DragonWord/Enemies/Component/BPC_Enemy_Health.BPC_Enemy_Health_C|GetDamage (Variables|Default|GetBPC_Enemy_Health)) 0 0))

(event Custom|MeleeHitBoxOff
  (Collision|SetCollisionEnabled (Variables|Default|GetMeleeAttackBox) "NoCollision"))

(event Custom|MeleeHitBoxOn
  (Collision|SetCollisionEnabled (Variables|Default|GetMeleeAttackBox) "QueryOnly"))

(event EventBeginPlay
  (|CallParentFunction)
  (CallFunction|SetEnemyType 0 self))

(event Collision|EventActorBeginOverlap
  (params (OtherActor :type Actor%20Object%20Reference))
  (|CallParentFunction OtherActor) ; This node is disabled and will not be called.\nDrag off pins to build functionality.
)

(event EventTick
  (params (DeltaSeconds :type Float%20%28single-precision%29))
  (|CallParentFunction DeltaSeconds) ; This node is disabled and will not be called.\nDrag off pins to build functionality.
)

(fn ConstructionScript
  (|CallParentFunction))