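; BP_Projectiles_Base is a projectile, apparently a base class, that damages the wizard player.
; It moves along a local offset every tick without sweep or delta-time scaling, and destroys itself after a ten-second lifetime.
; A custom hit event, not called within this file, applies fixed damage if the passed actor matches the BP_WizardPlayer found by class lookup, then destroys the projectile whatever it hit.
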(event Custom|PlayerDamgeProjectiles
  (params (Other%20Actor :type Object%20Object%20Reference))
  (Utilities|FlowControl|Sequence
    (:then_0
      (bind _returnvalue (Actor|GetActorOfClass "/Game/DragonWord/Player/BP_WizardPlayer.BP_WizardPlayer_C"))
      (if (== _returnvalue Other%20Actor)
        (Game|Damage|ApplyDamage _returnvalue 25.0 0 0)))
    (:then_1
      (Actor|DestroyActor))))

(event EventBeginPlay
  (Utilities|FlowControl|Delay 1e+01)
  (Actor|DestroyActor))

(event Collision|EventActorBeginOverlap
  (params (OtherActor :type Actor%20Object%20Reference)))

(event EventTick
  (params (DeltaSeconds :type Float%20%28single-precision%29))
  (Transformation|AddActorLocalOffset (Variables|Default|GetX%20Only) false false))

(fn ConstructionScript)